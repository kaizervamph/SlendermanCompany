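; Replicated grabbable loot item whose mesh, random starting price and fragility come from LootData.
; Hard impacts pass a gate, opened on grab and closed shortly after release, with a brief cooldown between hits.
; The server deducts fragility-scaled damage from the price, destroying the item at zero, while clients update price and damage widgets.
; A looping server timer also runs a debug-drawn sphere trace whose results go unused.
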(event OnComponentHit(StaticMesh)
  (params (HitComponent :type Primitive%20Component%20Object%20Reference) (OtherActor :type Actor%20Object%20Reference) (OtherComp :type Primitive%20Component%20Object%20Reference) (NormalImpulse :type Vector :default "0, 0, 0") (Hit :type Hit%20Result%20Structure%20%28by%20ref%29))
  (bind _returnvalue (Math|Vector|VectorLength NormalImpulse))
  (Networking|SwitchHasAuthority
    (:Authority
      (Utilities|Array|AddUnique (Variables|Default|GetHitComponents) HitComponent)
      (if (> _returnvalue 1.2e+03)
        (Utilities|FlowControl|Gate true :!label _label
          (:Exit
            (CallFunction|AllonDamage (Math|Float|Truncate (Math|Float|SafeDivide _returnvalue 1e+01)))
            (Utilities|FlowControl|Sequence
              (:then_0
                (Utilities|FlowControl|RetriggerableDelay 0.2)
                (goto _label Open))
              (:then_1
                (goto _label Close)))))))))

(event Custom|CheckCollidingComponents
  (bind _staticmesh (Variables|Default|GetStaticMesh))
  (bind (_origin _boxextent _sphereradius) (Collision|GetComponentBounds _staticmesh))
  (Collision|MultiSphereTraceByChannel _origin _origin _sphereradius "TraceTypeQuery1" false 0 "Persistent"))

(event Custom|All_UpdateIsGrabbed
  (params (Instigator :type Controller%20Object%20Reference) (NowGrabbed :type Boolean))
  (Networking|SwitchHasAuthority
    (:Remote
      (if (== Instigator (Game|GetPlayerController 0))
        (Rendering|SetVisibility (Variables|Default|GetPriceWidget) NowGrabbed false)
        (bind _aswbp_item_price (Utilities|Casting|CastToWBP_ItemPrice (UserInterface|GetWidget (Variables|Default|GetPriceWidget))))
        (Default|UpdatePrice _aswbp_item_price (Variables|Default|GetItemPrice))))))

(event Custom|All_OnDamage
  (params (Damage :type Integer))
  (bind _lootdata (Variables|Default|GetLootData)
    (:then
      (Development|PrintString (Utilities|String|ToString(Float) (Math|Float|SafeDivide (Variables|/Game/CoreGameplay/LootSystem/Looteables/DA_Looteable.DA_Looteable_C|GetFragility _lootdata) 1e+02)))
      (Networking|SwitchHasAuthority
        (:Authority
          (if (<= (- (Variables|Default|GetItemPrice) (Math|Float|Truncate (* Damage (Math|Float|SafeDivide (Variables|/Game/CoreGameplay/LootSystem/Looteables/DA_Looteable.DA_Looteable_C|GetFragility _lootdata) 1e+02)))) 0)
            (Actor|DestroyActor)
            (else
              (Variables|Default|SetItemPrice (- (Variables|Default|GetItemPrice) (Math|Float|Truncate (* Damage (Math|Float|SafeDivide (Variables|/Game/CoreGameplay/LootSystem/Looteables/DA_Looteable.DA_Looteable_C|GetFragility _lootdata) 1e+02))))))))
        (:Remote
          (bind _aswbp_item_price_damage_container (Utilities|Casting|CastToWBP_ItemPriceDamageContainer (UserInterface|GetWidget (Variables|Default|GetDamageWidget))))
          (Default|UpdatePrice _aswbp_item_price_damage_container (Math|Float|Truncate (* Damage (Math|Float|SafeDivide (Variables|/Game/CoreGameplay/LootSystem/Looteables/DA_Looteable.DA_Looteable_C|GetFragility _lootdata) 1e+02)))))))
    (:else)))

(event EventOnUpdateIsGrabbed
  (params (GrabInstigator :type Controller%20Object%20Reference) (NowGrabbed :type Boolean))
  (Networking|SwitchHasAuthority
    (:Authority
      (CallFunction|AllUpdateIsGrabbed GrabInstigator NowGrabbed)
      (if NowGrabbed
        (Utilities|FlowControl|Delay 0.1)
        (Utilities|FlowControl|Gate true) ; enters at Open
        (else
          (Utilities|FlowControl|Delay 1.0)
          (Utilities|FlowControl|Gate true) ; enters at Close
        )))))

(event EventBeginPlay
  (|CallParentFunction)
  (Networking|SwitchHasAuthority
    (:Authority
      (Utilities|FlowControl|Sequence
        (:then_0
          (bind _lootdata (Variables|Default|GetLootData)
            (:then
              (Variables|Default|SetItemPrice (Math|Float|Truncate (Math|Random|RandomFloatinRange (.X (Math|Vector2D|BreakVector2D (Variables|/Game/CoreGameplay/LootSystem/Looteables/DA_Looteable.DA_Looteable_C|GetPriceRange _lootdata))) (.Y (Math|Vector2D|BreakVector2D (Variables|/Game/CoreGameplay/LootSystem/Looteables/DA_Looteable.DA_Looteable_C|GetPriceRange _lootdata)))))))
            (:else)))
        (:then_1
          (Utilities|Time|SetTimerbyEvent (delegate Custom|CheckCollidingComponents) 0.02 true))))))

(fn ConstructionScript
  (|CallParentFunction)
  (CallFunction|UpdateMesh))

(fn OnRepLootData
  (CallFunction|UpdateMesh))

(fn UpdateMesh
  (bind _lootdata (Variables|Default|GetLootData)
    (:then
      (bind _mesh (Variables|/Game/CoreGameplay/LootSystem/Looteables/DA_Looteable.DA_Looteable_C|GetMesh _lootdata)
        (:then
          (Components|StaticMesh|SetStaticMesh (Variables|Default|GetStaticMesh) _mesh)
          (return))
        (:else)))
    (:else)))

(fn OnRepItemPrice
  (Networking|SwitchHasAuthority
    (:Remote
      (bind _aswbp_item_price (Utilities|Casting|CastToWBP_ItemPrice (UserInterface|GetWidget (Variables|Default|GetPriceWidget))))
      (Default|UpdatePrice _aswbp_item_price (Variables|Default|GetItemPrice)))))