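; BP_LootCarrier is a loot container that totals the price of the lootable items inside its Box volume.
; Begin and end overlaps on the Box call UpdatePrice, which on the authority sums ItemPrice across overlapping BP_LooteableItem actors into Price.
; The Price RepNotify shows the total as a dollar amount on TotalPrice text and prints it for debugging.
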(event OnComponentBeginOverlap(Box)
  (params (OverlappedComponent :type Primitive%20Component%20Object%20Reference) (OtherActor :type Actor%20Object%20Reference) (OtherComp :type Primitive%20Component%20Object%20Reference) (OtherBodyIndex :type Integer) (bFromSweep :type Boolean) (SweepResult :type Hit%20Result%20Structure%20%28by%20ref%29))
  (CallFunction|UpdatePrice))

(event OnComponentEndOverlap(Box)
  (params (OverlappedComponent :type Primitive%20Component%20Object%20Reference) (OtherActor :type Actor%20Object%20Reference) (OtherComp :type Primitive%20Component%20Object%20Reference) (OtherBodyIndex :type Integer))
  (CallFunction|UpdatePrice))

(fn ConstructionScript
  (|CallParentFunction))

(fn UpdatePrice
  (Networking|SwitchHasAuthority
    (:Authority
      (for _array_element (Collision|GetOverlappingActors (Variables|Default|GetBox) "/Game/CoreGameplay/LootSystem/BP_LooteableItem.BP_LooteableItem_C" :!class /Script/Engine.PrimitiveComponent)
        (bind _asbp_looteable_item (Utilities|Casting|CastToBP_LooteableItem _array_element))
        (LocalVariables|SetTemp (+ (Variables|/Game/CoreGameplay/LootSystem/BP_LooteableItem.BP_LooteableItem_C|GetItemPrice _asbp_looteable_item) (LocalVariables|GetTemp))))
      (Variables|Default|SetPrice (LocalVariables|GetTemp)))))

(fn OnRepPrice
  (bind _price (Variables|Default|GetPrice))
  (Rendering|Components|TextRender|SetText (Variables|Default|GetTotalPrice) (Utilities|Text|FormatText "${price}" _price))
  (Development|PrintString (Utilities|String|ToString(Integer) _price)))